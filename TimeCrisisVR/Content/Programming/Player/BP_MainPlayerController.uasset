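; VR player controller that handles teleport and node-based locomotion.
; While the empty hand's thumbstick is held, Tick traces a debug-drawn projectile arc in segments, highlighting any PlayerConstraintArea hit.
; Releasing on a valid target loads Main_Scene from the tutorial, otherwise updates the nav manager section directly, with a camera fade, or with forced HMD rotation, per GameInstance modifier.
; Node-based moves lerp the pawn along a timeline, with a separate rotation event.
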(event `self.MovePlayerViaNavManagerNodeBased`
  (bind (_locomotiontomovetowards_x _locomotiontomovetowards_y) (`KismetMathLibrary.BreakVector` (`self.LocomotionToMoveTowards`)))
  (bind (_returnvalue_x _returnvalue_y) (`KismetMathLibrary.BreakVector` (`self.K2_GetActorLocation` (`GameplayStatics.GetPlayerPawn` 0))))
  ;[1 1 1] Node Based Locomotion
  (bind (_direction _newtrack_4) (`Timeline|Point Transition` :!via `PlayFromStart`)
    (:`Update`
      (`self.K2_SetActorLocation` (`GameplayStatics.GetPlayerPawn` 0) (`KismetMathLibrary.VLerp` (`KismetMathLibrary.MakeVector` _returnvalue_x _returnvalue_y) (`KismetMathLibrary.MakeVector` _locomotiontomovetowards_x _locomotiontomovetowards_y) _newtrack_4) false false))))

(event `self.DrawTeleportArc`
  (bind _found_teleport_panel (`self.Found Teleport Panel`))
  (bind _found_teleport_panel_2 (`self.Found Teleport Panel`))
  ;[1 1 1] Parabola on the left hand
  (bind _asvrpawn (cast `VRPawn` (`GameplayStatics.GetPlayerPawn` 0)))
  (bind _returnvalue (`VRPawn.CheckWhichHandIsEmpty` _asvrpawn))
  (switch `EHand` _returnvalue
    (:`LEFT`
      (bind _mcleft (`VRPawn.MCLeft` _asvrpawn))
      (bind _returnvalue_2 (`SceneComponent.K2_GetComponentLocation` _mcleft))
      (bind _returnvalue_3 (`SceneComponent.K2_GetComponentRotation` _mcleft))
      (set `self.InitialVelocityWithRot` (`KismetMathLibrary.TransformDirection` (`KismetMathLibrary.MakeTransform` (+ _returnvalue_2 (`KismetMathLibrary.GreaterGreater_VectorRotator` _returnvalue_2 _returnvalue_3)) _returnvalue_3) (`self.PathPower`)))
      (bind _asvrpawn_2 (cast `VRPawn` (`GameplayStatics.GetPlayerPawn` 0)))
      (for _index (range (+ (`KismetMathLibrary.FFloor` (/ (`self.PathLifeTime`) (`self.TimeInterval`))) 1)) :!label _label
        (bind (_point_1 _point_2) (`self.GetSegmentAtTime` (`SceneComponent.K2_GetComponentLocation` (`VRPawn.MCLeft` _asvrpawn_2)) (`self.InitialVelocityWithRot`) (0.0 0.0 -980.0) (* _index (`self.TimeInterval`)) (* (+ _index 1) (`self.TimeInterval`))))
        (bind (_outhit _returnvalue_4) (`KismetSystemLibrary.LineTraceSingle` :`Start` _point_1 :`End` _point_2 :`TraceChannel` "TraceTypeQuery1" :`DrawDebugType` "ForOneFrame"))
        (if _returnvalue_4
          (bind _asplayer_constraint_area (cast `PlayerConstraintArea` (`.HitActor` (`GameplayStatics.BreakHitResult` _outhit)))
            (:`then`
              (set `self.Found Teleport Panel` _asplayer_constraint_area)
              (set `self.InValidSpace` true)
              (set `self.EndLocation` (`.Location` (`GameplayStatics.BreakHitResult` _outhit)))
              (`self.BreakDrawingLeft`)
              (`PlayerConstraintArea.ChangePanelColor` (`self.Found Teleport Panel`) true))
            (:`CastFailed`
              (set `self.InValidSpace` false)))
          (elif (!= _found_teleport_panel null)
            (`PlayerConstraintArea.ChangePanelColor` _found_teleport_panel false)))))
    (:`RIGHT`
      (bind _asvrpawn_3 (cast `VRPawn` (`GameplayStatics.GetPlayerPawn` 0)))
      (bind _mcright (`VRPawn.MCRight` _asvrpawn_3))
      (bind _returnvalue_5 (`SceneComponent.K2_GetComponentLocation` _mcright))
      (bind _returnvalue_6 (`SceneComponent.K2_GetComponentRotation` _mcright))
      ;[1 1 1] Parabola on the right hand
      (set `self.InitialVelocityWithRot` (`KismetMathLibrary.TransformDirection` (`KismetMathLibrary.MakeTransform` (+ _returnvalue_5 (`KismetMathLibrary.GreaterGreater_VectorRotator` _returnvalue_5 _returnvalue_6)) _returnvalue_6) (`self.PathPower`)))
      (bind _asvrpawn_4 (cast `VRPawn` (`GameplayStatics.GetPlayerPawn` 0)))
      (for _index_2 (range (+ (`KismetMathLibrary.FFloor` (/ (`self.PathLifeTime`) (`self.TimeInterval`))) 1)) :!label _label_2
        (bind (_point_1_2 _point_2_2) (`self.GetSegmentAtTime` (`SceneComponent.K2_GetComponentLocation` (`VRPawn.MCRight` _asvrpawn_4)) (`self.InitialVelocityWithRot`) (0.0 0.0 -980.0) (* _index_2 (`self.TimeInterval`)) (* (+ _index_2 1) (`self.TimeInterval`))))
        (bind (_outhit_2 _returnvalue_7) (`KismetSystemLibrary.LineTraceSingle` :`Start` _point_1_2 :`End` _point_2_2 :`TraceChannel` "TraceTypeQuery1" :`DrawDebugType` "ForOneFrame"))
        (if _returnvalue_7
          (bind _asplayer_constraint_area_2 (cast `PlayerConstraintArea` (`.HitActor` (`GameplayStatics.BreakHitResult` _outhit_2)))
            (:`then`
              (set `self.Found Teleport Panel` _asplayer_constraint_area_2)
              (set `self.InValidSpace` true)
              (set `self.EndLocation` (`.Location` (`GameplayStatics.BreakHitResult` _outhit_2)))
              (`self.BreakDrawingRight`)
              (`PlayerConstraintArea.ChangePanelColor` (`self.Found Teleport Panel`) true))
            (:`CastFailed`
              (set `self.InValidSpace` false)))
          (elif (!= _found_teleport_panel_2 null)
            (`PlayerConstraintArea.ChangePanelColor` _found_teleport_panel_2 false)))))))

(event `BreakDrawingLeft`
  ;[1 1 1] Parabola on the left hand
  (goto _label :!via `Break`))

(event `BreakDrawingRight`
  ;[1 1 1] Parabola on the right hand
  (goto _label_2 :!via `Break`))

(event `Key|MotionController_Left_Thumbstick`
  (params (Key :type "Key Structure"))
  (bind _returnvalue (and (== (`self.bAllowToTeleportThisGame`) true) (== (`self.bCanTeleportAfterAllEnemiesDead`) true)))
  ;[1 1 1] Does the enable and disable of pressing the right input etc and allows the navigation manager to update if the input is valid
  (:`Pressed`
    (if _returnvalue
      (bind _asvrpawn (cast `VRPawn` (`GameplayStatics.GetPlayerPawn` 0)))
      (bind _returnvalue_2 (`VRPawn.CheckWhichHandIsEmpty` _asvrpawn))
      (switch `EHand` _returnvalue_2
        (:`LEFT`
          (set `self.DidPressStick` true)))))
  (:`Released`
    (if _returnvalue
      (bind _asvrpawn_2 (cast `VRPawn` (`GameplayStatics.GetPlayerPawn` 0)))
      (bind _returnvalue_3 (`VRPawn.CheckWhichHandIsEmpty` _asvrpawn_2))
      (switch `EHand` _returnvalue_3
        (:`LEFT`
          (set `self.DidPressStick` false)
          (if (`self.InValidSpace`) :!label _label_3
            (set `self.InValidSpace` false)
            ;;[1 1 1] Get the right modifier type
            (bind _astutorial_to_game_save_instance (cast `TutorialToGameSaveInstance` (`GameplayStatics.GetGameInstance`))
              (:`then`
                (if (`self.bIsTutorial`)
                  (`GameplayStatics.OpenLevel` "Main_Scene")
                  (else
                    (bind _returnvalue_4 (`TutorialToGameSaveInstance.GetModifierType` _astutorial_to_game_save_instance))
                    (switch `EModifierTypes` _returnvalue_4
                      (:`NONE`
                        (`self.UpdateSectionViaNavManager`))
                      (:`FADE`
                        (`self.Fade_Point_And_Teleport`))
                      (:`FORCED_ROTATION`
                        (`self.Rotate Player On Arc Teleport` :!label _label_4))
                      (:`ANNOTATED_ROTATION`
                        (goto _label_4))))))
              (:`CastFailed`
                (`KismetSystemLibrary.PrintString` "Failed Cast")))))))))

(event `Key|MotionController_Right_Thumbstick`
  (params (Key :type "Key Structure"))
  (bind _returnvalue (and (== (`self.bAllowToTeleportThisGame`) true) (== (`self.bCanTeleportAfterAllEnemiesDead`) true)))
  ;[1 1 1] Does the enable and disable of pressing the right input etc and allows the navigation manager to update if the input is valid
  (:`Pressed`
    (if _returnvalue
      (bind _asvrpawn (cast `VRPawn` (`GameplayStatics.GetPlayerPawn` 0)))
      (bind _returnvalue_2 (`VRPawn.CheckWhichHandIsEmpty` _asvrpawn))
      (switch `EHand` _returnvalue_2
        (:`RIGHT`
          (set `self.DidPressStick` true)))))
  (:`Released`
    (if _returnvalue
      (bind _asvrpawn_2 (cast `VRPawn` (`GameplayStatics.GetPlayerPawn` 0)))
      (bind _returnvalue_3 (`VRPawn.CheckWhichHandIsEmpty` _asvrpawn_2))
      (switch `EHand` _returnvalue_3
        (:`RIGHT`
          (set `self.DidPressStick` false)
          (goto _label_3))))))

(event `self.ReceiveTick`
  (params (DeltaSeconds :type "Float (single-precision)"))
  ;[1 1 1] Allows the parabola to be drawn constantly
  (if (`self.DidPressStick`)
    (`self.DrawTeleportArc`)))

(event `self.RotatePlayerAfterTeleport`
  (bind _returnvalue (`GameplayStatics.GetPlayerController` 0))
  (bind _returnvalue_2 (* (.yaw (`self.RotationToFaceTowards`)) -1.0))
  ;[1 1 1] Forced Rotation
  ;;[1 1 1] This version is for Node based and appears in the code of the navigation manager
  (bind _asvr_pawn (cast `/Game/Programming/Player/VR_Pawn` (`GameplayStatics.GetPlayerPawn` 0)))
  (bind _vrcamera (`VRPawn.VRCamera` _asvr_pawn))
  (set `CameraComponent.bLockToHmd` false _vrcamera)
  (`OculusFunctionLibrary.SetBaseRotationAndBaseOffsetInMeters` (`KismetMathLibrary.MakeRotator` 0.0 0.0 _returnvalue_2) (0.0 0.0 0.0) "Orientation")
  (`self.SetControlRotation` _returnvalue (`KismetMathLibrary.ComposeRotators` (`KismetMathLibrary.MakeRotator` 0.0 0.0 _returnvalue_2) (`self.GetControlRotation` _returnvalue)))
  (set `CameraComponent.bLockToHmd` true _vrcamera))

(event `Rotate Player On Arc Teleport`
  (bind _returnvalue (`GameplayStatics.GetPlayerController` 0))
  (bind _returnvalue_2 (* (.yaw (`self.RotationToFaceTowards`)) -1.0))
  ;[1 1 1] Forced Rotation
  ;;[1 1 1] This version is for POINT AND TELEPORT AS IT UPDATES THE LOCATION
  (bind _asvr_pawn (cast `/Game/Programming/Player/VR_Pawn` (`GameplayStatics.GetPlayerPawn` 0)))
  (bind _vrcamera (`VRPawn.VRCamera` _asvr_pawn))
  (set `CameraComponent.bLockToHmd` false _vrcamera)
  (`OculusFunctionLibrary.SetBaseRotationAndBaseOffsetInMeters` (`KismetMathLibrary.MakeRotator` 0.0 0.0 _returnvalue_2) (0.0 0.0 0.0) "Orientation")
  (`self.SetControlRotation` _returnvalue (`KismetMathLibrary.ComposeRotators` (`KismetMathLibrary.MakeRotator` 0.0 0.0 _returnvalue_2) (`self.GetControlRotation` _returnvalue)))
  (`self.UpdateSectionViaNavManager`)
  (set `CameraComponent.bLockToHmd` true _vrcamera))

(fn `GetSegmentAtTime`
  (params (StartLocation :type "Vector Structure") (InitialVelocity :type "Vector Structure") (Gravity :type "Vector Structure") (`Time 1` :type "Float (double-precision)") (`Time 2` :type "Float (double-precision)"))
  (returns (`Point 1` :type "Vector Structure") (`Point 2` :type "Vector Structure"))
  (return (+ StartLocation (* InitialVelocity `Time 1`) (* Gravity (* `Time 1` `Time 1` 0.5))) (+ StartLocation (* InitialVelocity `Time 2`) (* Gravity (* `Time 2` `Time 2` 0.5)))))

(fn `SetUpBeam`
  (params (PawnObj :type "VRPawn Object Reference") (SourcePoint :type "Vector Structure") (TargetPoint :type "Vector Structure"))
  (bind _childactor (`self.ChildActor`))
  (bind _returnvalue (`self.GetComponentByClass` (`ChildActorComponent.ChildActor` _childactor) "/Script/Engine.SplineComponent"))
  (`SplineComponent.ClearSplinePoints` _returnvalue true)
  (bind _output_get (set `self.StartPnt` (make `SplinePoint` 0.0 SourcePoint (0.0 0.0 500.0))))
  (bind _output_get_2 (set `self.EndPnt` (make `SplinePoint` 0.0 TargetPoint (0.0 0.0 -500.0))))
  (`SplineComponent.AddPoints` _returnvalue (`|MakeArray` _output_get _output_get_2) true)
  (for _index (range (+ (- (`SplineComponent.GetNumberOfSplinePoints` _returnvalue) 2) 1))
    (bind _returnvalue_2 (`AddComponent|NODE_AddSplineMeshComponent-0` :`bManualAttachment` true))
    (`SceneComponent.K2_AttachToComponent` _returnvalue_2 _childactor "None" "KeepRelative" "KeepRelative" "KeepRelative" true)
    (bind (_location _tangent) (`SplineComponent.GetLocationAndTangentAtSplinePoint` _returnvalue _index "Local"))
    (bind (_location_2 _tangent_2) (`SplineComponent.GetLocationAndTangentAtSplinePoint` _returnvalue (+ _index 1) "Local"))
    (`SplineMeshComponent.SetStartAndEnd` _returnvalue_2 _location _tangent _location_2 _tangent_2 true)))

(fn `UserConstructionScript`)