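; BP_AmmoHolsters is the player's ammo holster actor, which smoothly follows the VR camera as a body-relative anchor.
; Each tick it interpolates toward a point behind and below the camera, rotating in yaw only.
; Yaw blends from the camera's forward vector to its up vector as the player looks down, keeping facing stable.
; Interpolation uses delta time divided by global time dilation, so following ignores slow motion.
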(event `self.ReceiveTick`
  (params (DeltaSeconds :type "Float (single-precision)"))
  (bind _returnvalue_location (`KismetMathLibrary.BreakTransform` (`self.GetTransform`)))
  ;[1 1 1] Used to set the correct rotation and location around the player object
  (bind _asvr_pawn (cast `/Game/Programming/Player/VR_Pawn` (`GameplayStatics.GetPlayerPawn` 0)))
  (bind _delta_time (`self.Get Delta Time Ignore Dilation`))
  (bind _delta_time_2 (`self.Get Delta Time Ignore Dilation`))
  (bind _vrcamera (`VRPawn.VRCamera` _asvr_pawn))
  (`self.K2_SetActorTransform` (`KismetMathLibrary.MakeTransform` (`KismetMathLibrary.VInterpTo` _returnvalue_location (`KismetMathLibrary.TransformLocation` (`SceneComponent.K2_GetComponentToWorld` _vrcamera) (-12.0 0.0 -5.0)) _delta_time 4.0) (`KismetMathLibrary.RInterpTo` (`SceneComponent.K2_GetComponentRotation` (`self.RootComp`)) (`KismetMathLibrary.MakeRotator` 0.0 0.0 (.yaw (`KismetMathLibrary.RLerp` (`KismetMathLibrary.MakeRotFromXZ` (`SceneComponent.GetUpVector` _vrcamera) (0.0 0.0 1.0)) (`KismetMathLibrary.MakeRotFromXZ` (`SceneComponent.GetForwardVector` _vrcamera) (0.0 0.0 1.0)) (`KismetMathLibrary.FClamp` (* (+ (/ (`KismetMathLibrary.DegAcos` (`KismetMathLibrary.Dot_VectorVector` (`SceneComponent.GetForwardVector` _vrcamera) (0.0 0.0 -1.0))) 90.0) -0.5) 3.0)) true))) _delta_time_2 8.0))))

(fn `Get Delta Time Ignore Dilation`
  (returns (`Delta Time` :type "Float (double-precision)"))
  (return (* (/ 1.0 (`GameplayStatics.GetGlobalTimeDilation`)) (`GameplayStatics.GetWorldDeltaSeconds`))))

(fn `UserConstructionScript`)